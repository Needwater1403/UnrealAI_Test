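; Attack component that gives its owning actor a projectile spell and an instant raycast attack.
; MagicSpell spawns a targeted dark energy projectile and binds its impact event, which deals damage and signals attack end.
; FireRaycast line-traces for Pawns and damages the hit actor, without signalling attack end.
; Both paths send damage through a TakeDamage message and report it to AI damage sensing.
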(event Custom|Magic%20Spell
  (params (SpawnTransform :type Transform) (Target :type Actor%20Object%20Reference) (DamageInfo :type S%20Damage%20Info%20Structure))
  (bind _returnvalue (Game|SpawnActorfromClass "/Game/Projectiles/BP_Projectile_DarkEnergy.BP_Projectile_DarkEnergy_C" SpawnTransform "Undefined" "MultiplyWithRoot" (Components|GetOwner) 1e+03 0.0 Target false 0))
  (EventDispatchers|AssignOnProjectileImpact _returnvalue (delegate Custom|OnProjectileImpact_Event))
  (Collision|IgnoreActorwhenMoving (Actor|GetComponentbyClass (Components|GetOwner) "/Script/Engine.CapsuleComponent") _returnvalue false))

(event Custom|OnProjectileImpact_Event
  (params (OtherActor :type Actor%20Object%20Reference) (Hit :type Hit%20Result%20Structure))
  (bind _returnvalue (Components|GetOwner))
  (Class|BPIDamagable|TakeDamage(Message) OtherActor (stale Custom|Magic%20Spell DamageInfo) _returnvalue)
  (Class|AISenseDamage|ReportDamageEvent OtherActor _returnvalue (.Amount (Utilities|Struct|BreakS_DamageInfo (stale Custom|Magic%20Spell DamageInfo))) (Transformation|GetActorLocation _returnvalue) "0, 0, 0" "None")
  (Default|CallOnAttackEnd))

(event Custom|FireRaycast
  (params (TraceStartPos :type Vector) (TraceEndPos :type Vector) (DamageInfo :type S%20Damage%20Info%20Structure))
  (bind _returnvalue (Components|GetOwner))
  (bind (_outhit _returnvalue_2) (Collision|LineTraceForObjects TraceStartPos TraceEndPos (Utilities|Array|MakeArray "ObjectTypeQuery3") false 0 "None"))
  (if _returnvalue_2
    (Class|BPIDamagable|TakeDamage(Message) (.HitActor (Collision|BreakHitResult _outhit)) DamageInfo _returnvalue)
    (Class|AISenseDamage|ReportDamageEvent (.HitActor (Collision|BreakHitResult _outhit)) _returnvalue (.Amount (Utilities|Struct|BreakS_DamageInfo DamageInfo)) (Transformation|GetActorLocation _returnvalue) "0, 0, 0" "None")))