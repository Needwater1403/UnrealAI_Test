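; BP_Enemy_Base is the base enemy character, with health, an overhead health bar widget and AI-driven states.
; Health, healing and damage are delegated to a damage system component, whose death event ragdolls the mesh, sets the AI controller dead and hides the bar.
; A hit reaction stops movement, freezes the AI during a montage, then returns it to combat against the damage dealer.
; Getters expose patrol route, ideal ranges and movement-speed presets.
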(event Custom|Event%20Death
  (bind _mesh (Variables|Character|GetMesh))
  ;[1 1 1] RAGDOLL
  (Physics|SetSimulatePhysics _mesh true)
  (Collision|SetCollisionEnabled _mesh "QueryAndPhysics")
  (Default|SetStateasDead (Variables|Default|GetAICEnemyBase))
  (Default|HideVisibility (Variables|Default|GetHPBarWidget)))

(event Custom|OnDamageResponse_Event
  (params (DamageResponse :type E_DamageResponse%20Enum :default "NewEnumerator0") (DamageDealer :type Actor%20Object%20Reference))
  (bind _aicenemybase (Variables|Default|GetAICEnemyBase))
  (switch Utilities|FlowControl|Switch|SwitchonE_DamageResponse DamageResponse
    (:NewEnumerator1
      (Components|Movement|StopMovementImmediately (Variables|Character|GetCharacterMovement))
      (Default|SetStateasFrozen _aicenemybase)
      (Animation|Montage|PlayMontage (Variables|Character|GetMesh) (Variables|AnimMontage|GetHit%20Montage%20to%20Play)
        (:OnCompleted
          (Development|PrintString "Hello"))
        (:OnInterrupted
          _))
      (Default|SetStateasCombat _aicenemybase DamageDealer))))

(event EventBeginPlay
  (bind _bpc_damagesystem (Variables|Default|GetBPC_DamageSystem))
  ;[1 1 1] Bind Event
  (EventDispatchers|BindEventtoOnDeath _bpc_damagesystem (EventDispatchers|CreateEvent :!event Custom|Event%20Death))
  (EventDispatchers|AssignOnDamageResponse _bpc_damagesystem (EventDispatchers|CreateEvent :!event Custom|OnDamageResponse_Event))
  ;[1 1 1] Create HP Bar Widget
  (bind _returnvalue (UserInterface|CreateWidget "/Game/DamageSystem/W_HealthBar.W_HealthBar_C" 0 self))
  (UserInterface|SetWidget (Variables|Default|GetHPBar) _returnvalue)
  (Variables|Default|SetHPBarWidget _returnvalue)
  (bind _asaic_enemy_base (Utilities|Casting|CastToAIC_Enemy_Base (AI|GetAIController self)))
  (Variables|Default|SetAICEnemyBase _asaic_enemy_base))

(fn ConstructionScript)

(fn GetCurrentHealth
  (return (Variables|/Game/DamageSystem/BPC_DamageSystem.BPC_DamageSystem_C|GetHealth (Variables|Default|GetBPC_DamageSystem))))

(fn GetIdealRange
  (return 2e+02 3.5e+02))

(fn GetMaxHealth
  (return (Variables|/Game/DamageSystem/BPC_DamageSystem.BPC_DamageSystem_C|GetMaxHealth (Variables|Default|GetBPC_DamageSystem))))

(fn GetPatrolRoute
  (return (Variables|Default|GetpatrolRoute)))

(fn Heal
  (params (Amount :type Float%20%28double-precision%29))
  (bind _newhealth (Default|Heal (Variables|Default|GetBPC_DamageSystem) Amount))
  (return _newhealth))

(fn IsAttacking
  (return (Variables|Default|GetAttacking)))

(fn IsDead
  (return (Variables|/Game/DamageSystem/BPC_DamageSystem.BPC_DamageSystem_C|GetIsDead (Variables|Default|GetBPC_DamageSystem))))

(fn SetMovementSpeed
  (params (movementType :type E_MovementSpeed%20Enum :default "NewEnumerator0"))
  (bind _output_get (Variables|/Script/Engine.CharacterMovementComponent|SetMaxWalkSpeed (Variables|Character|GetCharacterMovement) (Utilities|Select :Index movementType :NewEnumerator0 0.0 :NewEnumerator1 2e+02 :NewEnumerator2 5e+02 :NewEnumerator4 5.5e+02 :NewEnumerator5 1e+02)))
  (return _output_get))

(fn TakeDamage
  (params (DamageInfo :type S%20Damage%20Info%20Structure) (Dealer :type Actor%20Object%20Reference))
  (bind _wasdamaged (Default|TakeDamage (Variables|Default|GetBPC_DamageSystem) DamageInfo Dealer))
  (return _wasdamaged))