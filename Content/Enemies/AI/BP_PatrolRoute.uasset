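; BP_PatrolRoute defines a patrol path for enemy AI using the points of a Route spline.
; IncrementPatrolRoute steps PatrolPointIndex by Direction, reversing at the first and last points so the index ping-pongs along the spline.
; GetSplinePointAsWorldPos returns the world location of the current point.
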(event Custom|IncrementPatrolRoute
  (bind _output_get (Variables|Default|SetPatrolPointIndex (+ (Variables|Default|GetPatrolPointIndex) (Variables|Default|GetDirection))))
  (if (== _output_get (- (Spline|GetNumberOfSplinePoints (Variables|Default|GetRoute)) 1))
    (Variables|Default|SetDirection -1)
    (elif (== (Variables|Default|GetPatrolPointIndex) 0)
      (Variables|Default|SetDirection 1))))

(fn ConstructionScript)

(fn GetSplinePointasWorldPos
  (return (Spline|GetLocationatSplinePoint (Variables|Default|GetRoute) (Variables|Default|GetPatrolPointIndex) "World")))