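; BP_Enemy_Range is a ranged rifle enemy that extends a parent enemy Blueprint.
; On BeginPlay it spawns a rifle, attaches it to the hand socket and signals that a weapon is wielded.
; Attack plays the fire montage, whose notify fires a damage raycast running from the AI controller's current target back to the weapon, then signals attack end.
; Overrides supply movement speed per movement type and ideal attack and defense ranges.
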(event EventBeginPlay
  (|CallParentFunction)
  (bind _returnvalue (Game|SpawnActorfromClass "/Game/Weapons/BP_Weapon_Rifle.BP_Weapon_Rifle_C" (Transformation|GetActorTransform) "Undefined" "MultiplyWithRoot" 0 0))
  (bind _output_get (Variables|Default|SetWeaponActor _returnvalue))
  (Transformation|AttachComponentToComponent _output_get (Variables|Character|GetMesh) "hand_r_rifle_socket" "SnapToTarget" "SnapToTarget" "SnapToTarget" true)
  (Variables|Default|SetIsWieldingWeapon true)
  (Default|CallOnWieldWeapon))

(event EventAttack
  (Variables|Default|SetAttacking true)
  (bind _notifyname (Animation|Montage|PlayMontage (Variables|Character|GetMesh) "/Game/Animations/Rifle/Montage_Rifle_Fire.Montage_Rifle_Fire")
    (:OnCompleted
      (Default|CallOnAttackEnd :!label _label)
      (Variables|Default|SetAttacking false))
    (:OnInterrupted
      (goto _label))
    (:OnNotifyBegin
      (switch name _notifyname
        (:Fire
          (bind _asaic_enemy_base (Utilities|Casting|CastToAIC_Enemy_Base (AI|GetAIController self)))
          (Default|FireRaycast (Variables|Default|GetBPC_AttackMove) (Transformation|GetActorLocation (Variables|/Game/Enemies/AI/AIC_Enemy_Base.AIC_Enemy_Base_C|GetCurrentTarget _asaic_enemy_base)) (Transformation|GetActorLocation (Variables|Default|GetWeaponActor)) (Utilities|Struct|MakeS_DamageInfo 25.0 "NewEnumerator2" "NewEnumerator1")))))))

(fn ConstructionScript
  (|CallParentFunction))

(fn SetMovementSpeed
  (params (movementType :type E_MovementSpeed%20Enum :default "NewEnumerator0"))
  (bind _output_get (Variables|/Script/Engine.CharacterMovementComponent|SetMaxWalkSpeed (Variables|Character|GetCharacterMovement) (Utilities|Select :Index movementType :NewEnumerator0 0.0 :NewEnumerator1 2e+02 :NewEnumerator2 3e+02 :NewEnumerator4 5e+02 :NewEnumerator5 1e+02)))
  (return _output_get))

(fn GetIdealRange
  (return 6.5e+02 6.5e+02))