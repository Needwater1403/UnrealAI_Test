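; Melee enemy child Blueprint that fights with a spear, spawned at BeginPlay, attached to the right hand socket and registered with the combat system.
; Attack, wield and sheathe events play montages, then fire end callbacks whether completed or interrupted.
; Blocking stops movement and flags the damage system, whose OnBlocked event triggers a reaction montage.
; A block state enum keeps that reaction from ending the block early when it interrupts the block montage.
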(event Custom|StartBlock
  ;[1 1 1] BLOCK
  (Components|Movement|StopMovementImmediately (Variables|Character|GetCharacterMovement))
  (Variables|/Game/DamageSystem/BPC_DamageSystem.BPC_DamageSystem_C|SetIsBlocking (Variables|Default|GetBPC_DamageSystem) true)
  (Variables|Default|SetBlockState "NewEnumerator1")
  (Animation|Montage|PlayMontage (Variables|Character|GetMesh) "/Game/Animations/Melee/Montage_Sword_Block.Montage_Sword_Block"
    (:OnCompleted
      (CallFunction|FinishBlock :!label _label))
    (:OnInterrupted
      (if (Utilities|Enum|NotEqual(Enum) (Variables|Default|GetBlockState) "NewEnumerator2")
        (goto _label)))))

(event Custom|Assign%20Event
  (EventDispatchers|AssignOnBlocked (Variables|Default|GetBPC_DamageSystem) (EventDispatchers|CreateEvent :!event Custom|OnBlocked_Event)))

(event Custom|OnBlocked_Event
  (params (CanBeParried :type Boolean))
  ;[1 1 1] BLOCK
  (Variables|Default|SetBlockState "NewEnumerator2")
  (Animation|Montage|PlayMontage (Variables|Character|GetMesh) "/Game/Animations/Melee/Montage_Sword_Block_React.Montage_Sword_Block_React"
    (:OnCompleted
      _)
    (:OnInterrupted
      _))
  (CallFunction|FinishBlock))

(event Custom|FinishBlock
  ;[1 1 1] BLOCK
  (Variables|/Game/DamageSystem/BPC_DamageSystem.BPC_DamageSystem_C|SetIsBlocking (Variables|Default|GetBPC_DamageSystem) false)
  (Variables|Default|SetBlockState "NewEnumerator0")
  (Default|CallOnBlockEnd))

(event EventBeginPlay
  (|CallParentFunction)
  (CallFunction|AssignEvent)
  (bind _returnvalue (Game|SpawnActorfromClass "/Game/Weapons/BP_Weapon_Spear.BP_Weapon_Spear_C" (Transformation|GetActorTransform) "Undefined" "MultiplyWithRoot" 0 0))
  (bind _output_get (Variables|Default|SetWeaponActor _returnvalue))
  (Transformation|AttachComponentToComponent _output_get (Variables|Character|GetMesh) "hand_r_weapon_socket" "SnapToTarget" "SnapToTarget" "SnapToTarget" true)
  (Variables|/Game/Combat/BP_CombatSystem.BP_CombatSystem_C|SetWeaponActor (Variables|Default|GetBP_CombatSystem) _returnvalue))

(event EventAttack
  (Animation|Montage|PlayMontage (Variables|Character|GetMesh) "/Game/Animations/SpearAnimationsV2/Animations/Character/2Hand/Pose01/Spear_Thrust_Low_2H.Spear_Thrust_Low_2H"
    (:OnCompleted
      _)
    (:OnInterrupted
      _))
  (Default|CallOnAttackEnd))

(event EventSheatWeapon
  ;[1 1 1] Wield And Sheat
  (Animation|Montage|PlayMontage (Variables|Character|GetMesh) "/Game/Animations/ReTargetSpear/A_2H01_to_1H02_Montage.A_2H01_to_1H02_Montage"
    (:OnCompleted
      _)
    (:OnInterrupted
      _))
  (Default|CallOnSheathWeapon)
  (Variables|Default|SetIsWieldingWeapon false))

(event EventWieldWeapon
  ;[1 1 1] Wield And Sheat
  (Variables|Default|SetIsWieldingWeapon true)
  (Animation|Montage|PlayMontage (Variables|Character|GetMesh) "/Game/Animations/ReTargetSpear/A_1H02_to_2H01_Montage.A_1H02_to_2H01_Montage"
    (:OnCompleted
      _)
    (:OnInterrupted
      _))
  (Default|CallOnWieldWeapon))

(fn ConstructionScript
  (|CallParentFunction))