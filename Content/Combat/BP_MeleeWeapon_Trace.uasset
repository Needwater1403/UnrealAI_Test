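; Anim notify state that opens and closes the melee weapon trace window during attack animations.
; On begin, it casts the mesh owner to BP_Player or BP_Enemy_Base and calls StartMeleeWeaponTrace on its BPCombatSystem.
; On end, it resolves the owner the same way and calls StopWeaponTrace.
; The tracing itself is delegated to the combat system component, so player and enemies share one notify.
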(fn ReceivedNotifyBegin
  (params (MeshComp :type Skeletal%20Mesh%20Component%20Object%20Reference) (Animation :type Anim%20Sequence%20Base%20Object%20Reference) (TotalDuration :type Float%20%28single-precision%29) (EventReference :type Anim%20Notify%20Event%20Reference%20Structure%20%28by%20ref%29))
  (bind _returnvalue (Components|GetOwner MeshComp))
  (bind _asbp_player (Utilities|Casting|CastToBP_Player _returnvalue)
    (:then
      (Default|StartMeleeWeaponTrace (Variables|/Game/Player/BP_Player.BP_Player_C|GetBP_CombatSystem _asbp_player))
      (return false))
    (:CastFailed
      (bind _asbp_enemy_base (Utilities|Casting|CastToBP_Enemy_Base _returnvalue)
        (:then
          (Default|StartMeleeWeaponTrace (Variables|/Game/Enemies/BP_Enemy_Base.BP_Enemy_Base_C|GetBP_CombatSystem _asbp_enemy_base))
          (return false))
        (:CastFailed
          (return false))))))

(fn ReceivedNotifyEnd
  (params (MeshComp :type Skeletal%20Mesh%20Component%20Object%20Reference) (Animation :type Anim%20Sequence%20Base%20Object%20Reference) (EventReference :type Anim%20Notify%20Event%20Reference%20Structure%20%28by%20ref%29))
  (bind _returnvalue (Components|GetOwner MeshComp))
  (bind _asbp_player (Utilities|Casting|CastToBP_Player _returnvalue)
    (:then
      (Default|StopWeaponTrace (Variables|/Game/Player/BP_Player.BP_Player_C|GetBP_CombatSystem _asbp_player))
      (return false))
    (:CastFailed
      (bind _asbp_enemy_base (Utilities|Casting|CastToBP_Enemy_Base _returnvalue))
      (Default|StopWeaponTrace (Variables|/Game/Enemies/BP_Enemy_Base.BP_Enemy_Base_C|GetBP_CombatSystem _asbp_enemy_base))
      (return false))))