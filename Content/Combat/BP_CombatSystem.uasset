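; Combat system Blueprint that runs melee weapon hit detection and deals damage for its owner.
; Start and stop events control a fast looping timer that sphere-traces for Pawns between the weapon actor's start and end points, with debug drawing.
; A hit sends a TakeDamage message carrying a fixed damage struct and the owner as dealer.
; A DoOnce reset after a short delay throttles repeat hits across all targets.
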(event Custom|Start%20Melee%20Weapon%20Trace
  (bind _returnvalue (Utilities|Time|SetTimerbyEvent (delegate Custom|Loop%20Melee%20Weapon%20Trace) 0.02 true))
  (Variables|Default|SetWeaponTraceLoop _returnvalue))

(event Custom|Loop%20Melee%20Weapon%20Trace
  (bind (_outhit _returnvalue) (Collision|SphereTraceForObjects (Transformation|GetWorldLocation (Variables|/Game/Weapons/BP_Weapon_Base.BP_Weapon_Base_C|GetTraceStartPoint (Variables|Default|GetWeaponActor))) (Transformation|GetWorldLocation (Variables|/Game/Weapons/BP_Weapon_Base.BP_Weapon_Base_C|GetTraceEndPoint (Variables|Default|GetWeaponActor))) 12.0 (Utilities|Array|MakeArray "ObjectTypeQuery3") false 0 "ForDuration" true "(R=1.000000,G=0.000000,B=0.000000,A=1.000000)" "(R=0.000000,G=1.000000,B=0.000000,A=1.000000)" 0.2))
  (if _returnvalue
    (Utilities|FlowControl|DoOnce false :!label _label
      (:Completed
        (Class|BPIDamagable|TakeDamage(Message) (.HitActor (Collision|BreakHitResult _outhit)) (Utilities|Struct|MakeS_DamageInfo 5e+01 "NewEnumerator1") (Components|GetOwner))
        (Utilities|FlowControl|Delay 0.5)
        (goto _label Reset)))))

(event Custom|Stop%20Weapon%20Trace
  (Utilities|Time|ClearandInvalidateTimerbyHandle (Variables|Default|GetWeaponTraceLoop)))